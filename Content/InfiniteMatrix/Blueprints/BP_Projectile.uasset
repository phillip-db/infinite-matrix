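; BP_Projectile is the player's short-lived shot that destroys enemies and awards score.
; Each tick it moves along world X at a multiple of the player's ForwardSpeed, so it outpaces the player.
; On overlap with a BP_Enemy it adds score to the player and destroys both the enemy and itself.
; Overlaps with the player are ignored, any other actor destroys it, and it expires after a brief lifespan.
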(event `self.ReceiveBeginPlay`
  (`self.SetLifeSpan` 2.0))

(event `self.ReceiveActorBeginOverlap`
  (params (OtherActor :type "Actor Object Reference"))
  (bind _asbp_enemy (cast `/Game/InfiniteMatrix/Blueprints/BP_Enemy` OtherActor)
    (:`then`
      (bind _asbp_player (cast `/Game/InfiniteMatrix/Blueprints/BP_Player` (`GameplayStatics.GetPlayerPawn` 0)))
      (`/Game/InfiniteMatrix/Blueprints/BP_Player.UpdateScore` _asbp_player 5)
      (`self.K2_DestroyActor` _asbp_enemy)
      (`self.K2_DestroyActor`))
    (:`CastFailed`
      (cast `/Game/InfiniteMatrix/Blueprints/BP_Player` OtherActor
        (:`CastFailed`
          (`self.K2_DestroyActor`))))))

(event `self.ReceiveTick`
  (params (DeltaSeconds :type "Float (single-precision)"))
  (bind _asbp_player (cast `/Game/InfiniteMatrix/Blueprints/BP_Player` (`GameplayStatics.GetPlayerPawn` 0))
    (:`then`
      (`self.K2_AddActorWorldOffset` (`KismetMathLibrary.MakeVector` (* (* (`/Game/InfiniteMatrix/Blueprints/BP_Player.ForwardSpeed` _asbp_player) 1.5) DeltaSeconds))))
    (:`CastFailed`
      (`KismetSystemLibrary.PrintString` "Cast failed!"))))

(fn `UserConstructionScript`)